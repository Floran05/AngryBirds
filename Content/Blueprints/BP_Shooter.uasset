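; BP_Shooter is a ball-throwing shooter Blueprint that drives the in-game HUD and throw animation.
; It creates WBP_InGame on BeginPlay, then updates its power gauge and remaining-ball count through OnPowerChanged and OnShoot.
; Each shot briefly pulses IsThrowing on the goalie throw AnimBlueprint.
; When no balls remain, it swaps the HUD for WBP_End and switches to UI-only input.
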(event EventBeginPlay
  (bind _returnvalue (UserInterface|CreateWidget "/Game/UI/WBP_InGame.WBP_InGame_C" (Game|GetPlayerController 0)))
  (bind _output_get (Variables|Default|SetW_InGame _returnvalue))
  (UserInterface|Viewport|AddtoViewport _output_get 0))

(event Collision|EventActorBeginOverlap
  (params (OtherActor :type Actor%20Object%20Reference)))

(event EventTick
  (params (DeltaSeconds :type Float%20%28single-precision%29)))

(event EventOnShoot
  (bind _returnvalue (Class|AShooter|GetRemainingBalls))
  (bind _returnvalue_2 (Game|GetPlayerController 0))
  (Default|SetRemainingBalls (Variables|Default|GetW_InGame) _returnvalue)
  (bind _asgoalie_throw_skeleton_anim_blueprint (Utilities|Casting|CastToGoalie_Throw_Skeleton_AnimBlueprint (Components|SkeletalMesh|GetAnimInstance (Variables|Default|GetSkeletalMesh))))
  (Variables|/Game/Assets/Player/Goalie_Throw_Skeleton_AnimBlueprint.Goalie_Throw_Skeleton_AnimBlueprint_C|SetIsThrowing _asgoalie_throw_skeleton_anim_blueprint true)
  (Utilities|FlowControl|Delay 0.2)
  (Variables|/Game/Assets/Player/Goalie_Throw_Skeleton_AnimBlueprint.Goalie_Throw_Skeleton_AnimBlueprint_C|SetIsThrowing _asgoalie_throw_skeleton_anim_blueprint false)
  (if (< _returnvalue 1)
    (bind _returnvalue_3 (UserInterface|CreateWidget "/Game/UI/WBP_End.WBP_End_C" _returnvalue_2))
    (UserInterface|Viewport|AddtoViewport _returnvalue_3 0)
    (Widget|RemovefromParent (Variables|Default|GetW_InGame))
    (Input|SetInputModeUIOnly _returnvalue_2 _returnvalue_3 "DoNotLock" false)))

(event EventOnPowerChanged
  (params (Power :type Float%20%28single-precision%29))
  (Default|SetPowerPurcent (Variables|Default|GetW_InGame) Power 1.0))

(fn ConstructionScript)